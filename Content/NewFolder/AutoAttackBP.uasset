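; AutoAttackBP is an actor that automatically spawns a MagicBP actor on a looping two-second timer.
; BeginPlay starts the timer, and each firing spawns MagicBP at the actor's own location and rotation.
; Tick turns the Arrow component to face player pawn 0, but the spawn transform does not use that rotation.
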(event `self.ReceiveBeginPlay`
  (`KismetSystemLibrary.K2_SetTimerDelegate` (delegate `on_time`) 2.0 true))

(event `on_time`
  (`|SpawnActorFromClass` "/Game/NewFolder/MagicBP.MagicBP_C" (`KismetMathLibrary.MakeTransform` (`self.K2_GetActorLocation`) (`self.K2_GetActorRotation`)) "Undefined" "OverrideRootScale" null null))

(event `self.ReceiveTick`
  (params (DeltaSeconds :type "Float (single-precision)"))
  (`SceneComponent.K2_SetWorldRotation` (`self.Arrow`) (`KismetMathLibrary.MakeRotFromX` (- (`self.K2_GetActorLocation` (`GameplayStatics.GetPlayerPawn` 0)) (`self.K2_GetActorLocation`))) false false))

(fn `UserConstructionScript`)